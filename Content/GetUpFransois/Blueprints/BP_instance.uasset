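; BP_instance holds the game's scoreboard as an array of timed entries and records the index of the last score added.
; AddToScoreboard loops to insert a new time, but compares each element's Time with itself, so insertion never triggers.
; The fallback append runs only when ScoreAdded is true.
; SaveGame is never called and only reassigns the scoreboard to itself, leaving CurrentSaveGame unused.
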(fn AddtoScoreboard
  (params (New%20Time :type Struct%20Scoreboard%20Structure))
  (bind _structscoreboard (Variables|Default|GetstructScoreboard))
  (bind (_array_element _array_index) (Utilities|Array|ForEachLoopwithBreak _structscoreboard :!label _label)
    (:LoopBody
      (if (> (Utilities|Struct|BreakStruct_Scoreboard _array_element) (Utilities|Struct|BreakStruct_Scoreboard _array_element))
        (Utilities|Array|Insert _structscoreboard New%20Time _array_index)
        (Variables|Default|SetLasr%20score%20added _array_index)
        (Variables|Default|SetScore%20added true)
        (goto _label Break)))
    (:Completed
      (if (Variables|Default|GetScore%20added)
        (bind _returnvalue (Utilities|Array|Add (Variables|Default|GetstructScoreboard) New%20Time))
        (Variables|Default|SetLasr%20score%20added _returnvalue)))))

(fn SaveGame
  (Variables|Default|SetstructScoreboard (Variables|Default|GetstructScoreboard)))