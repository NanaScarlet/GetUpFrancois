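; AC_Health is an actor component that tracks health for the actor that owns it.
; On BeginPlay it binds to the owner's OnTakeAnyDamage event.
; The damage handler subtracts incoming damage, clamps Health between zero and HealthMax, then fires the Damage dispatcher, followed by Death whenever Health is zero.
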(event EventBeginPlay
  (EventDispatchers|BindEventtoOnTakeAnyDamage (Components|GetOwner) (EventDispatchers|CreateEvent :!event ACHealthAutoGenFunc)))

(event EventTick
  (params (DeltaSeconds :type Float%20%28single-precision%29)))

(fn ACHealthAutoGenFunc
  (params (DamagedActor :type Actor%20Object%20Reference) (Damage :type Float%20%28single-precision%29) (DamageType :type Damage%20Type%20Object%20Reference) (InstigatedBy :type Controller%20Object%20Reference) (DamageCauser :type Actor%20Object%20Reference))
  (bind _output_get (Variables|Default|SetHealth (Math|Float|Clamp(Float) (- (Variables|Default|GetHealth) Damage) 0.0 (Variables|Default|GetHealthMax))))
  (Default|CallDamage)
  (if (== _output_get 0.0)
    (Default|CallDeath)))