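; BP_SwapStates is an actor with Sad and Happy overlap zones that change the player's mood and handle reaching the win screen.
; Each zone sets BP_Player's FranMood and refreshes its flipbooks.
; Happy also waits briefly, shows WBP_youmadeit with the elapsed time, disables input and hides the cursor.
; A looping timer from BeginPlay counts seconds while GmeEnded is false, a flag this graph never sets.
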(event OnComponentBeginOverlap(Sad)
  (params (OverlappedComponent :type Primitive%20Component%20Object%20Reference) (OtherActor :type Actor%20Object%20Reference) (OtherComp :type Primitive%20Component%20Object%20Reference) (OtherBodyIndex :type Integer) (bFromSweep :type Boolean) (SweepResult :type Hit%20Result%20Structure%20%28by%20ref%29))
  (bind _asbp_player (Utilities|Casting|CastToBP_Player OtherActor))
  (Variables|/Game/GetUpFransois/Blueprints/BP_Player.BP_Player_C|SetFranMood _asbp_player "NewEnumerator0")
  (Default|SetFlipbooks _asbp_player))

(event OnComponentBeginOverlap(Happy)
  (params (OverlappedComponent :type Primitive%20Component%20Object%20Reference) (OtherActor :type Actor%20Object%20Reference) (OtherComp :type Primitive%20Component%20Object%20Reference) (OtherBodyIndex :type Integer) (bFromSweep :type Boolean) (SweepResult :type Hit%20Result%20Structure%20%28by%20ref%29))
  (bind _returnvalue (Game|GetPlayerController 0))
  (bind _asbp_player (Utilities|Casting|CastToBP_Player OtherActor))
  (Variables|/Game/GetUpFransois/Blueprints/BP_Player.BP_Player_C|SetFranMood _asbp_player "NewEnumerator2")
  (Default|SetFlipbooks _asbp_player)
  (Utilities|FlowControl|Delay 1.0)
  (bind _returnvalue_2 (UserInterface|CreateWidget "/Game/GetUpFransois/Widgets/WBP_youmadeit.WBP_youmadeit_C" 0 (Variables|Default|GetTime)))
  (UserInterface|Viewport|AddtoViewport _returnvalue_2 0)
  (Input|DisableInput (Game|GetPlayerCharacter 0) _returnvalue)
  (Variables|/Script/Engine.PlayerController|SetbShowMouseCursor _returnvalue false))

(event Custom|Count
  (if (not (Variables|Default|GetGme%20Ended))
    (Variables|Default|SetTime (+ (Variables|Default|GetTime) 1))))

(event Collision|EventActorBeginOverlap
  (params (OtherActor :type Actor%20Object%20Reference)))

(event EventTick
  (params (DeltaSeconds :type Float%20%28single-precision%29)))

(event EventBeginPlay
  (Utilities|Time|SetTimerbyEvent (delegate Custom|Count) 1.0 true))

(fn ConstructionScript)